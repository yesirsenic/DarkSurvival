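; BP_Monster is a zombie enemy that chases the player and attacks in melee.
; Every Tick reissues AI MoveTo, switches between Running and Attacking by distance, adjusts walk speed and copies IsAttacking from AnimBP_Monster.
; Hand capsule overlaps damage BP_Player during attacks, limited to one hit until AttackEndState resets the flag.
; Death plays a sound and destroys the actor.
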(event `self.ReceiveTick`
  (params (DeltaSeconds :type "Float (single-precision)"))
  (`|AIMoveTo` self (0.0 0.0 0.0) (`GameplayStatics.GetPlayerPawn` 0)
    (:`then`
      (`self.AttackAccess`)
      (`self.AttackSpeed`)
      (`self.AttackingCheck`))))

(event `self.RightHandCapsuleCollision.OnComponentBeginOverlap`
  (params (OverlappedComponent :type "PrimitiveComponent Object Reference") (OtherActor :type "Actor Object Reference") (OtherComp :type "PrimitiveComponent Object Reference") (OtherBodyIndex :type Integer) (bFromSweep :type Boolean) (SweepResult :type "HitResult Structure (by ref)"))
  (`self.PlayerAttacking` OtherActor))

(event `self.LeftHandCapsuleCollision.OnComponentBeginOverlap`
  (params (OverlappedComponent :type "PrimitiveComponent Object Reference") (OtherActor :type "Actor Object Reference") (OtherComp :type "PrimitiveComponent Object Reference") (OtherBodyIndex :type Integer) (bFromSweep :type Boolean) (SweepResult :type "HitResult Structure (by ref)"))
  (`self.PlayerAttacking` OtherActor))

(fn `AttackAccess`
  (if (> (`self.AttackRange`) (`self.GetDistanceTo` self (`GameplayStatics.GetPlayerPawn` 0)))
    (`self.SetState` "Attacking")
    (else
      (bind _asanim_bp_monster (cast `/Game/Resources/Monster/Anim/AnimBP/AnimBP_Monster` (`SkeletalMeshComponent.GetAnimInstance` (`self.Mesh`))))
      (if (not (`/Game/Resources/Monster/Anim/AnimBP/AnimBP_Monster.IsAttacking` _asanim_bp_monster))
        (`self.SetState` "Running")))))

(fn `AttackEndState`
  (set `self.AttackDamageEnd` false)
  (if (> (`self.AttackRange`) (`self.GetDistanceTo` self (`GameplayStatics.GetPlayerPawn` 0)))
    (`self.SetState` "Attacking")
    (else
      (`self.SetState` "Running"))))

(fn `AttackingCheck`
  (bind _asanim_bp_monster (cast `/Game/Resources/Monster/Anim/AnimBP/AnimBP_Monster` (`SkeletalMeshComponent.GetAnimInstance` (`self.Mesh`))))
  (set `self.IsAttacking` (`/Game/Resources/Monster/Anim/AnimBP/AnimBP_Monster.IsAttacking` _asanim_bp_monster)))

(fn `AttackSpeed`
  (if (`|EnumEquality` (`self.CharacterState`) "Attacking")
    (set `CharacterMovementComponent.MaxWalkSpeed` 0.0 (`self.CharacterMovement`))
    (elif (`|EnumEquality` (`self.CharacterState`) "Running")
      (set `CharacterMovementComponent.MaxWalkSpeed` 150.0 (`self.CharacterMovement`)))))

(fn `Death`
  (`GameplayStatics.PlaySound2D` "/Game/Resources/Sound/SFX/Zombie_Death_Cue.Zombie_Death_Cue" 1.0 1.0 0.0 null null)
  (`self.K2_DestroyActor`))

(fn `PlayerAttacking`
  (params (Object :type "Object Object Reference"))
  (bind _asbp_player (cast `/Game/BluePrints/Pure/BP_Player` Object))
  (if (and (`self.IsAttacking`) (not (`self.AttackDamageEnd`)))
    (`/Game/BluePrints/Pure/BP_Player.PlayerDamaged` _asbp_player)
    (set `self.AttackDamageEnd` true)))

(fn `UserConstructionScript`)